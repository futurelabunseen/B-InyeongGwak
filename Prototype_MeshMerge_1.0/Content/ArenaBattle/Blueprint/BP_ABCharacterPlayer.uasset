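; Player character Blueprint for ArenaBattle that adds a toggleable customizer screen.
; On BeginPlay it creates the B_CustomizerUI widget, adds it to the viewport and keeps it hidden.
; The V key runs a FlipFlop that shows the widget while slowing global time dilation to a near standstill, then hides it and restores normal speed.
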(event EventBeginPlay
  (bind _returnvalue (UserInterface|CreateWidget "/Game/ArenaBattle/ModuleParts/B_CustomizerUI.B_CustomizerUI_C"))
  (bind _output_get (Variables|Default|SetNewVar _returnvalue))
  (UserInterface|Viewport|AddtoViewport _output_get 0)
  (Widget|SetVisibility _output_get "Hidden"))

(event Collision|EventActorBeginOverlap
  (params (OtherActor :type Actor%20Object%20Reference)))

(event EventTick
  (params (DeltaSeconds :type Float%20%28single-precision%29)))

(event Input|KeyboardEvents|V
  (params (Key :type Key%20Structure :default "None"))
  (:Pressed
    (Utilities|FlowControl|FlipFlop
      (:A
        (Utilities|Time|SetGlobalTimeDilation 0.001)
        (Widget|SetVisibility (Variables|Default|GetNewVar) "Visible"))
      (:B
        (Utilities|Time|SetGlobalTimeDilation 1.0)
        (Widget|SetVisibility (Variables|Default|GetNewVar) "Hidden")))))

(fn ConstructionScript)