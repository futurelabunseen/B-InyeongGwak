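; Heavy homing missile projectile for Flight Suit 1 that launches with its shooter's velocity and accelerates forward through per-tick physics velocity interpolation.
; After firing, it searches a frontal cone for a tagged target every quarter second, then turns toward it at a timeline-ramped rate.
; Server-handled hits and overlaps, or a lifetime timer, trigger an explosion that sphere-traces for radius damage, multicasts effects and destroys the missile.
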(event OnComponentBeginOverlap(Missile)
  (params (OverlappedComponent :type Primitive%20Component%20Object%20Reference) (OtherActor :type Actor%20Object%20Reference) (OtherComp :type Primitive%20Component%20Object%20Reference) (OtherBodyIndex :type Integer) (bFromSweep :type Boolean) (SweepResult :type Hit%20Result%20Structure%20%28by%20ref%29))
  (bind _returnvalue (Components|GetOwner))
  (bind _missile (Variables|Default|GetMissile))
  (bind _returnvalue_2 (Transformation|GetWorldLocation _missile))
  ;[1 1 1] Hit effect
  (if (Networking|IsServer)
    (Utilities|IsValid _returnvalue
      (:Is%20Valid
        (bind _ignore_actors (Class|FS1BPI|GetIgnores(Message) _returnvalue))
        (if (not (Utilities|Array|ContainsItem _ignore_actors OtherActor))
          (if (Variables|Default|GetFired) :!label _label
            (Variables|Default|SetHit%20Target OtherActor)
            (if (not (Actor|ActorHasTag (stale Collision|EventHit _output_get) "projectile"))
              (bind _outhits (Collision|MultiSphereTraceForObjects _returnvalue_2 (+ _returnvalue_2 "0, 0,1.000000") (Variables|Default|GetBlast%20Radius) (Utilities|Array|MakeArray "ObjectTypeQuery1" "ObjectTypeQuery2" "ObjectTypeQuery3" "ObjectTypeQuery5" "ObjectTypeQuery6") false 0 "None"))
              (CallFunction|MulticastHitEffect _returnvalue_2)
              (for _array_element _outhits
                (Utilities|IsValid (.hitactor _array_element)
                  (:Is%20Valid
                    (Game|Damage|ApplyDamage (.hitactor _array_element) (Variables|Default|GetMissile%20Damage) (Game|GetInstigatorController) self))))
              (Actor|DestroyActor)))))
      (:Is%20Not%20Valid
        (goto _label)))))

(event Custom|Multicast%20Hit%20Effect
  (params (Location :type Vector))
  ;[1 1 1] Hit effect
  (CallFunction|FS1HitEffect (Variables|Default|GetExplosion%20Particle) (Variables|Default|GetExplosion%20Sound) Location "10.000000,10.000000,10.000000" 1.0 0.7 "/Game/Flight_Suit_1/Audio/200M_Attenuation.200M_Attenuation"))

(event Custom|Multicast%20Launch%20Effects
  ;[1 1 1] Fire and launch event
  (Components|Activation|Activate (Variables|Default|GetAudio) false)
  (Audio|SpawnSoundAttached "/Game/Flight_Suit_1/Audio/FS1_Missile_Fire_1_Cue.FS1_Missile_Fire_1_Cue" (Variables|Default|GetMissile) "None" "0, 0, 0" "0, 0, 0" "KeepRelativeOffset" false 1.0 0.6 0.0 "/Game/Flight_Suit_1/Audio/200M_Attenuation.200M_Attenuation" 0))

(event Custom|Explode
  (bind _missile (Variables|Default|GetMissile))
  (bind _returnvalue (Transformation|GetWorldLocation _missile))
  ;[1 1 1] Hit effect
  (bind _outhits (Collision|MultiSphereTraceForObjects _returnvalue (+ _returnvalue "0, 0,1.000000") (Variables|Default|GetBlast%20Radius) (Utilities|Array|MakeArray "ObjectTypeQuery1" "ObjectTypeQuery2" "ObjectTypeQuery3" "ObjectTypeQuery5" "ObjectTypeQuery6") false 0 "None"))
  (CallFunction|MulticastHitEffect _returnvalue)
  (for _array_element _outhits
    (Utilities|IsValid (.hitactor _array_element)
      (:Is%20Valid
        (Game|Damage|ApplyDamage (.hitactor _array_element) (Variables|Default|GetMissile%20Damage) (Game|GetInstigatorController) self))))
  (Actor|DestroyActor))

(event EventFS1UpdateMaterial
  (params (Armor :type Material%20Interface%20Object%20Reference) (Armor_2 :type Material%20Interface%20Object%20Reference) (Wings :type Material%20Interface%20Object%20Reference) (Minigun :type Material%20Interface%20Object%20Reference) (Railgun :type Material%20Interface%20Object%20Reference) (Rails :type Material%20Interface%20Object%20Reference) (Missiles :type Material%20Interface%20Object%20Reference))
  (Rendering|Material|SetMaterial (Variables|Default|GetMissile) 0 Missiles))

(event EventTick
  (params (DeltaSeconds :type Float%20%28single-precision%29))
  (bind _returnvalue (Transformation|GetVelocity))
  (bind _missile (Variables|Default|GetMissile))
  (bind _missile_2 (Variables|Default|GetMissile))
  ;[1 1 1] Update movement tick events
  (Physics|SetPhysicsLinearVelocity _missile (Math|Interpolation|VInterptoConstant (Math|Vector|SelectVector (Transformation|GetVelocity (Variables|Default|GetVelocity%20Source)) _returnvalue (Math|Vector|Equal(Vector) _returnvalue "0, 0, 0" 1e+01)) (Math|Vector|RotateVector "25000.000000, 0, 0" (Transformation|GetActorRotation)) DeltaSeconds 9e+03) false "None")
  (Class|PrimitiveComponent|SetPhysicsAngularVelocityinDegrees _missile (Math|Interpolation|VInterptoConstant (Physics|GetPhysicsAngularVelocityinDegrees _missile "None") "0, 0, 0" DeltaSeconds 1e+03) false "None")
  (if (Variables|Default|GetSeeking%20After%20Target)
    (Transformation|SetWorldRotation _missile_2 (Class|KismetMathLibrary|RInterptoConstant (Transformation|GetWorldRotation _missile_2) (Math|Rotator|FindLookatRotation (Transformation|GetActorLocation) (Transformation|GetActorLocation (Variables|Default|GetTarget))) (Utilities|Time|GetWorldDeltaSeconds) (Math|Float|Clamp(Float) (* 1.5e+02 (Variables|Default|GetHoming%20Lerp)) 1e-05 1.5e+02)) false false)))

(event Collision|EventHit
  (params (MyComp :type Primitive%20Component%20Object%20Reference) (Other :type Actor%20Object%20Reference) (OtherComp :type Primitive%20Component%20Object%20Reference) (bSelfMoved :type Boolean) (HitLocation :type Vector :default "0, 0, 0") (HitNormal :type Vector :default "0, 0, 0") (NormalImpulse :type Vector :default "0, 0, 0") (Hit :type Hit%20Result%20Structure%20%28by%20ref%29))
  (bind _missile (Variables|Default|GetMissile))
  (bind _returnvalue (Transformation|GetWorldLocation _missile))
  ;[1 1 1] Hit effect
  (if (Networking|IsServer)
    (bind _output_get (Variables|Default|SetHit%20Target Other))
    (if (Variables|Default|GetFired)
      (if (not (Actor|ActorHasTag _output_get "projectile"))
        (bind _outhits (Collision|MultiSphereTraceForObjects _returnvalue (+ _returnvalue "0, 0,1.000000") (Variables|Default|GetBlast%20Radius) (Utilities|Array|MakeArray "ObjectTypeQuery1" "ObjectTypeQuery2" "ObjectTypeQuery3" "ObjectTypeQuery5" "ObjectTypeQuery6") false 0 "None"))
        (CallFunction|MulticastHitEffect _returnvalue)
        (for _array_element _outhits
          (Utilities|IsValid (.hitactor _array_element)
            (:Is%20Valid
              (Game|Damage|ApplyDamage (.hitactor _array_element) (Variables|Default|GetMissile%20Damage) (Game|GetInstigatorController) self))))
        (Actor|DestroyActor)))))

(event EventFS1Fire
  (params (Firing%20Held :type Boolean) (Firing%20Mode%20Update :type Boolean) (Ready%20Firing :type Boolean) (Camera%20Reference :type Scene%20Component%20Object%20Reference) (Slots%20Affected%20By%20Fire :type FS1_Weapon_Slots_Enum%20Enum :default "NewEnumerator0") (Targeting%20Tag :type Name :default "None"))
  ;[1 1 1] Fire and launch event
  (Variables|Default|SetTarget%20Tag Targeting%20Tag)
  (Physics|SetPhysicsLinearVelocity (Variables|Default|GetMissile) (Transformation|GetVelocity (Components|GetOwner Camera%20Reference)) false "None")
  (Components|Activation|Activate (Variables|Default|GetAudio) false)
  (Variables|Default|SetFired true)
  (Utilities|FlowControl|Sequence
    (:then_0
      (bind (_target_found _target) (CallFunction|FS1FindTargetinFrontalCone self (Variables|Default|GetTarget%20Tag) 2e+04 3e+01 :!label _label))
      (if _target_found
        (Variables|Default|SetTarget _target)
        (Variables|Default|SetSeeking%20After%20Target true)
        (bind _newtrack_0 (Timeline|Timeline_0 PlayFromStart)
          (:Update
            (Variables|Default|SetHoming%20Lerp _newtrack_0)))
        (else
          (Utilities|FlowControl|Delay 0.25)
          (goto _label))))
    (:then_1
      (Utilities|Time|SetTimerbyEvent (delegate Custom|Explode) 1e+01)
      (CallFunction|MulticastLaunchEffects))))

(fn ConstructionScript)

(fn GetIgnores
  (return 0))