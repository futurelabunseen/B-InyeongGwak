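; Railgun round projectile for Flight Suit 1 that damages what it strikes and then destroys itself, with a particle trail attached on spawn.
; Hit and mesh overlap events are handled only on the server and share one damage path.
; Overlaps skip the owner's ignore list and actors tagged as projectiles.
; A multicast event plays the blue spark and impact sound at the round's location.
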(event OnComponentBeginOverlap(StaticMesh)
  (params (OverlappedComponent :type Primitive%20Component%20Object%20Reference) (OtherActor :type Actor%20Object%20Reference) (OtherComp :type Primitive%20Component%20Object%20Reference) (OtherBodyIndex :type Integer) (bFromSweep :type Boolean) (SweepResult :type Hit%20Result%20Structure%20%28by%20ref%29))
  (bind _returnvalue (Components|GetOwner))
  (if (Networking|IsServer)
    (Utilities|IsValid _returnvalue
      (:Is%20Valid
        (bind _ignore_actors (Class|FS1BPI|GetIgnores(Message) _returnvalue))
        (if (not (Utilities|Array|ContainsItem _ignore_actors OtherActor))
          (Variables|Default|SetHit%20Target OtherActor :!label _label)
          (if (not (Actor|ActorHasTag (stale Collision|EventHit _output_get) "projectile"))
            (Game|Damage|ApplyDamage (stale Collision|EventHit _output_get) (Variables|Default|GetBullet%20damage) (Game|GetInstigatorController) self)
            (CallFunction|MulticastHitEffect (Transformation|GetActorLocation))
            (Utilities|IsValid (stale EventBeginPlay _returnvalue)
              (:Is%20Valid
                (Components|DestroyComponent (stale EventBeginPlay _returnvalue)))
              (:Is%20Not%20Valid
                _))
            (Actor|DestroyActor))))
      (:Is%20Not%20Valid
        (goto _label)))))

(event Custom|Multicast%20Hit%20Effect
  (params (Location :type Vector))
  (CallFunction|FS1HitEffect "/Game/Flight_Suit_1/Particles/FS1_Hit_Spark_Blue_PS.FS1_Hit_Spark_Blue_PS" "/Game/Flight_Suit_1/Audio/Hit_Random_Cue.Hit_Random_Cue" Location "1.000000,1.000000,1.000000" 1.4 0.7 "/Game/Flight_Suit_1/Audio/200M_Attenuation.200M_Attenuation"))

(event EventBeginPlay
  (bind _returnvalue (Effects|SpawnEmitterAttached "/Game/Flight_Suit_1/Particles/FS1_Railgun_Trail_PS.FS1_Railgun_Trail_PS" (Variables|Default|GetStaticMesh) "None" "0, 0, 0" "0, 0, 0" "0.200000,0.200000,0.200000" "SnapToTarget")))

(event EventTick
  (params (DeltaSeconds :type Float%20%28single-precision%29)))

(event Collision|EventHit
  (params (MyComp :type Primitive%20Component%20Object%20Reference) (Other :type Actor%20Object%20Reference) (OtherComp :type Primitive%20Component%20Object%20Reference) (bSelfMoved :type Boolean) (HitLocation :type Vector :default "0, 0, 0") (HitNormal :type Vector :default "0, 0, 0") (NormalImpulse :type Vector :default "0, 0, 0") (Hit :type Hit%20Result%20Structure%20%28by%20ref%29))
  (if (Networking|IsServer)
    (bind _output_get (Variables|Default|SetHit%20Target Other))
    (Game|Damage|ApplyDamage _output_get (Variables|Default|GetBullet%20damage) (Game|GetInstigatorController) self)
    (CallFunction|MulticastHitEffect (Transformation|GetActorLocation))
    (Utilities|IsValid (stale EventBeginPlay _returnvalue)
      (:Is%20Valid
        (Components|DestroyComponent (stale EventBeginPlay _returnvalue)))
      (:Is%20Not%20Valid
        _))
    (Actor|DestroyActor)))

(fn ConstructionScript)