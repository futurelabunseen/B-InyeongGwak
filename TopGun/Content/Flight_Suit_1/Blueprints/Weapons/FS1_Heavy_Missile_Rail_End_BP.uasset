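; Heavy missile rail end weapon for Flight Suit 1 that carries and launches a single heavy missile.
; On fire it hides the mounted missile mesh and the server spawns a missile actor at that transform, passing it the camera, target tag and material.
; A fired flag blocks further launches until reload restores the mesh.
; Update events swap materials and toggle outlined meshes on the rail and missile.
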(event EventBeginPlay
  ;[1 1 1] Set weapon material on start
  (Rendering|Material|CreateDynamicMaterialInstance (Variables|Default|GetFS1_Heavy_Rail_End_SM) 0 0 "None" :!class /Script/Engine.PrimitiveComponent))

(event EventFS1Reload
  (params (Weapon%20To%20Reload :type FS1_Weapon_Slots_Enum%20Enum :default "NewEnumerator0"))
  ;[1 1 1] Reload Rail
  (Rendering|SetVisibility (Variables|Default|GetMissile_SM) true false)
  (Variables|Default|SetMissile%20Fired false))

(event EventTick
  (params (DeltaSeconds :type Float%20%28single-precision%29))
  ;[1 1 1] Animate glowing barrels
)

(event EventFS1Fire
  (params (Firing%20Held :type Boolean) (Firing%20Mode%20Update :type Boolean) (Ready%20Firing :type Boolean) (Camera%20Reference :type Scene%20Component%20Object%20Reference) (Slots%20Affected%20By%20Fire :type FS1_Weapon_Slots_Enum%20Enum :default "NewEnumerator0") (Targeting%20Tag :type Name :default "None"))
  (bind _missile_sm (Variables|Default|GetMissile_SM))
  ;[1 1 1] Recieve updates to fire
  (bind _output_get (Variables|Default|SetFiring%20Is%20Held Firing%20Held))
  (Variables|Default|SetReadied%20To%20Fire Ready%20Firing)
  (bind _output_get_2 (Variables|Default|SetTarget%20Tag Targeting%20Tag))
  ;[1 1 1] Spawn Missile
  (if _output_get
    (if (not (Variables|Default|GetMissile%20Fired))
      (Variables|Default|SetMissile%20Fired true)
      (Rendering|SetVisibility _missile_sm false false)
      (if (Networking|IsServer)
        (bind _returnvalue (Game|SpawnActorfromClass "/Game/Flight_Suit_1/Blueprints/Weapons/Projectiles/FS1_Missile_Heavy_BP.FS1_Missile_Heavy_BP_C" (Transformation|GetWorldTransform _missile_sm) "AlwaysSpawn" self "/Game/Flight_Suit_1/Demo/Particles/P_Explosion_PS.P_Explosion_PS" "/Game/Flight_Suit_1/Demo/Audio/Explosion_Cue.Explosion_Cue" (Components|GetOwner Camera%20Reference) 0))
        (Class|FS1BPI|FS1Fire(Message) _returnvalue true false false Camera%20Reference "NewEnumerator9" _output_get_2)
        (Class|FS1BPI|FS1UpdateMaterial(Message) _returnvalue 0 0 0 0 0 0 (Variables|Default|GetMissiles%20Mat))))))

(event EventFS1UpdateMaterial
  (params (Armor :type Material%20Interface%20Object%20Reference) (Armor_2 :type Material%20Interface%20Object%20Reference) (Wings :type Material%20Interface%20Object%20Reference) (Minigun :type Material%20Interface%20Object%20Reference) (Railgun :type Material%20Interface%20Object%20Reference) (Rails :type Material%20Interface%20Object%20Reference) (Missiles :type Material%20Interface%20Object%20Reference))
  (bind _fs1_heavy_rail_end_sm (Variables|Default|GetFS1_Heavy_Rail_End_SM))
  ;[1 1 1] Recieve updates to material
  (Variables|Default|SetMissiles%20Mat Missiles)
  (Rendering|Material|SetMaterial _fs1_heavy_rail_end_sm 0 Minigun)
  (Rendering|Material|CreateDynamicMaterialInstance _fs1_heavy_rail_end_sm 0 Minigun "None" :!class /Script/Engine.PrimitiveComponent)
  (Rendering|Material|SetMaterial (Variables|Default|GetMissile_SM) 0 Missiles))

(event EventFS1OutlinedMeshes
  (params (Use%20Outlined%20Meshes :type Boolean))
  ;[1 1 1] Update to outlined meshes
  (Components|StaticMesh|SetStaticMesh (Variables|Default|GetFS1_Heavy_Rail_End_SM) (select Use%20Outlined%20Meshes "/Game/Flight_Suit_1/Meshes/Weapons/Outlined/FS1_Heavy_Rail_End_Outlined_SM.FS1_Heavy_Rail_End_Outlined_SM" "/Game/Flight_Suit_1/Meshes/Weapons/FS1_Heavy_Rail_End_SM.FS1_Heavy_Rail_End_SM"))
  (Components|StaticMesh|SetStaticMesh (Variables|Default|GetMissile_SM) (select Use%20Outlined%20Meshes "/Game/Flight_Suit_1/Meshes/Weapons/Outlined/FS1_Heavy_Missile_Outlined_SM.FS1_Heavy_Missile_Outlined_SM" "/Game/Flight_Suit_1/Meshes/Weapons/FS1_Heavy_Missile_SM.FS1_Heavy_Missile_SM")))

(fn ConstructionScript)

(fn GetIgnores
  (bind _ignore_actors (Class|FS1BPI|GetIgnores(Message) (Components|GetOwner)))
  (return _ignore_actors))