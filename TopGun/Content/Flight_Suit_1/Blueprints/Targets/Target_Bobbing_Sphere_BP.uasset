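; Target sphere actor that bobs up and down around its spawn location and flashes when damaged.
; A timeline started on BeginPlay offsets Z by its curve times VerticalRange and restarts itself on finish to loop.
; AnyDamage calls HitEffectMulticast, which swaps the sphere to a glowing red material, then restores plain red after a short retriggerable delay.
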(event Custom|Hit%20Effect%20Multicast
  (bind _sphere (Variables|Default|GetSphere))
  (Rendering|Material|SetMaterial _sphere 0 "/Game/Flight_Suit_1/Materials/Targets/Red_Glow_M.Red_Glow_M")
  (Utilities|FlowControl|RetriggerableDelay 0.2)
  (Rendering|Material|SetMaterial _sphere 0 "/Game/Flight_Suit_1/Materials/Targets/Red_M.Red_M"))

(event EventBeginPlay
  (Variables|Default|SetStarting%20Location (Transformation|GetActorLocation))
  (bind _newtrack_0 (Timeline|Move%20Timeline PlayFromStart)
    (:Update
      (Transformation|SetActorLocation (Math|Vector|MakeVector (.x (Variables|Default|GetStarting%20Location)) (.y (Variables|Default|GetStarting%20Location)) (+ (.z (Variables|Default|GetStarting%20Location)) (* _newtrack_0 (Variables|Default|GetVertical%20Range)))) false false))
    (:Finished
      (Utilities|FlowControl|Sequence
        (:then_0
          (Timeline|Move%20Timeline PlayFromStart))))))

(event Collision|EventActorBeginOverlap
  (params (OtherActor :type Actor%20Object%20Reference)))

(event EventTick
  (params (DeltaSeconds :type Float%20%28single-precision%29)))

(event Game|Damage|EventAnyDamage
  (params (Damage :type Float%20%28single-precision%29) (DamageType :type Damage%20Type%20Object%20Reference) (InstigatedBy :type Controller%20Object%20Reference) (DamageCauser :type Actor%20Object%20Reference))
  (CallFunction|HitEffectMulticast))

(fn ConstructionScript)