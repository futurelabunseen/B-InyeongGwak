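; Blueprint function library for the Flight Suit asset, providing shared aiming, targeting and impact-effect helpers.
; FS1_Trace_Check line-traces far along a camera component's forward vector, returning the impact point, or the trace end on a miss.
; FS1_Find_Target_In_Frontal_Cone scans tagged actors within lock-on range, picking the one with the smallest angle from the actor's forward vector inside the field of view.
; FS1_Hit_Effect spawns an emitter and positional sound at a location.
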(fn FS1TraceCheck
  (params (Trace%20From%20Camera :type Scene%20Component%20Object%20Reference) (ActorsToIgnore :type Array%20of%20Actor%20Object%20References) (TraceChannel :type ETraceTypeQuery%20Enum :default "TraceTypeQuery1"))
  (bind _returnvalue (Transformation|GetWorldLocation Trace%20From%20Camera))
  (bind _returnvalue_2 (Math|Vector|GetForwardVector Trace%20From%20Camera))
  (bind _returnvalue_3 (* _returnvalue_2 999999999))
  (bind _returnvalue_4 (+ _returnvalue _returnvalue_3))
  (bind (_outhit _returnvalue_5) (Collision|LineTraceByChannel 0 _returnvalue _returnvalue_4 TraceChannel false ActorsToIgnore "None"))
  (return (select _returnvalue_5 (.ImpactPoint (Collision|BreakHitResult _outhit)) _returnvalue_4) _returnvalue_5 (.HitActor (Collision|BreakHitResult _outhit)) _outhit))

(fn FS1FindTargetinFrontalCone
  (params (Targeting%20Actor%20%28Self%29 :type Actor%20Object%20Reference) (Search%20Tag :type Name :default "target") (Lock%20On%20Range :type Float%20%28single-precision%29) (Lock%20On%20Field%20Of%20View :type Float%20%28single-precision%29))
  (LocalVariables|SetLowest_FoV Lock%20On%20Field%20Of%20View)
  (bind _outactors (Actor|GetAllActorswithTag 0 Search%20Tag))
  (for _array_element _outactors
    (if (<= (Math|Vector|VectorLength (- (Transformation|GetActorLocation _array_element) (Transformation|GetActorLocation Targeting%20Actor%20%28Self%29))) Lock%20On%20Range)
      (if (< (Class|KismetMathLibrary|DegAcos (Math|Vector|DotProduct (Math|Vector|Normalize (- (Transformation|GetActorLocation _array_element) (Transformation|GetActorLocation Targeting%20Actor%20%28Self%29))) (Math|Vector|Normalize (Transformation|GetActorForwardVector Targeting%20Actor%20%28Self%29)))) (LocalVariables|GetLowest_FoV))
        (LocalVariables|SetCurrent%20Best%20Target _array_element)
        (LocalVariables|SetLowest_FoV (Class|KismetMathLibrary|DegAcos (Math|Vector|DotProduct (Math|Vector|Normalize (- (Transformation|GetActorLocation _array_element) (Transformation|GetActorLocation Targeting%20Actor%20%28Self%29))) (Math|Vector|Normalize (Transformation|GetActorForwardVector Targeting%20Actor%20%28Self%29)))))
        (LocalVariables|SetValid%20Target%20Found true))))
  (return (LocalVariables|GetValid%20Target%20Found) (LocalVariables|GetCurrent%20Best%20Target)))

(fn FS1HitEffect
  (params (EmitterTemplate :type Particle%20System%20Object%20Reference) (Sound :type Sound%20Base%20Object%20Reference) (Location :type Vector) (Scale :type Vector :default "1.000000,1.000000,1.000000") (VolumeMultiplier :type Float%20%28single-precision%29) (PitchMultiplier :type Float%20%28single-precision%29) (AttenuationSettings :type Sound%20Attenuation%20Object%20Reference) (ConcurrencySettings :type Sound%20Concurrency%20Object%20Reference))
  (Effects|SpawnEmitteratLocation 0 EmitterTemplate Location "0, 0, 0" Scale)
  (Audio|SpawnSoundatLocation 0 Sound Location "0, 0, 0" VolumeMultiplier PitchMultiplier 0.0 AttenuationSettings ConcurrencySettings))