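; Weapon preview actor for the weapon customization screen, acting as the player's view target.
; On BeginPlay it creates the six-slot customization widget, adds it to the viewport, passes it a self reference and switches player 0's view to itself.
; SetCamera performs the same view switch on demand.
; Clicking the actor or its Cube sets CanRotate, though this Blueprint's graphs contain no rotation logic.
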(event OnClicked(Cube)
  (params (TouchedComponent :type Primitive%20Component%20Object%20Reference) (ButtonPressed :type Key%20Structure))
  (Variables|Default|SetCanRotate? true))

(event Custom|SetCamera
  (Game|Player|SetViewTargetwithBlend (Game|GetPlayerController 0) self 0.0 "VTBlend_Linear" 0.0 true))

(event EventBeginPlay
  (bind _returnvalue (UserInterface|CreateWidget "/Game/DUWepCustSys/BluePrints/UI/WBP_6CustWepSlots.WBP_6CustWepSlots_C"))
  (bind _output_get (Variables|Default|SetWBP_6CustSlots _returnvalue))
  (UserInterface|Viewport|AddtoViewport _output_get 0)
  (Variables|/Game/DUWepCustSys/BluePrints/UI/WBP_6CustWepSlots.WBP_6CustWepSlots_C|SetAct_WepPreview (Variables|Default|GetWBP_6CustSlots) self)
  (Game|Player|SetViewTargetwithBlend (Game|GetPlayerController 0) self 0.0 "VTBlend_Linear" 0.0 true))

(event MouseInput|EventActorOnClicked
  (params (ButtonPressed :type Key%20Structure))
  (Variables|Default|SetCanRotate? true))

(fn ConstructionScript)