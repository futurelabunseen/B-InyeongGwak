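; Podded minigun weapon that fires a stream of spread bullets while the fire input is held.
; A re-arming timer paces shots, spawning bullet actors on the server with attached muzzle effects and fading firing audio.
; Tick eases a barrel heat glow on a dynamic material and nudges the muzzle arrow toward the targeting camera's trace point.
; Fire state is forwarded to the anim instance, and events swap outlined meshes and materials.
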(event Custom|Next%20Round%20Ready
  (bind _arrow (Variables|Default|GetArrow))
  (bind _returnvalue (Transformation|GetWorldTransform _arrow))
  ;[1 1 1] Fire bullets
  (if (Variables|Default|GetFiring)
    (if (Networking|IsServer)
      (Game|SpawnActorfromClass "/Game/Flight_Suit_1/Blueprints/Weapons/Projectiles/FS1_Bullet_BP.FS1_Bullet_BP_C" (Math|Transform|MakeTransform (.location _returnvalue) (Math|Conversions|RotationFromXVector (Math|Random|RandomUnitVectorinConeinDegrees (Math|Vector|GetForwardVector _arrow) (Variables|Default|GetBullet%20Spread))) (.scale _returnvalue)) "AlwaysSpawn" "OverrideRootScale" self 0))
    (Effects|SpawnEmitterAttached "/Game/Flight_Suit_1/Particles/Bullet_Firing_PS.Bullet_Firing_PS" (Variables|Default|GetArrow) "None" "0, 0, 0" "0, 0, 0" "0.200000,0.200000,0.200000")
    (Utilities|Time|SetTimerbyEvent (delegate Custom|Next%20Round%20Ready) (/ 1.0 (Variables|Default|GetBullets%20Per%20Second)))))

(event EventBeginPlay
  (bind _weapon_mesh (Variables|Default|GetWeapon_Mesh))
  ;[1 1 1] Set weapon material on start
  (bind _returnvalue (Rendering|Material|CreateDynamicMaterialInstance _weapon_mesh 0 0 "None" :!class /Script/Engine.PrimitiveComponent))
  (bind _output_get (Variables|Default|SetMaterial%20Inst _returnvalue))
  (Rendering|Material|SetScalarParameterValue _output_get "Emis Power" (Variables|Default|GetGlow) :!class /Script/Engine.MaterialInstanceDynamic)
  (Variables|Default|SetGun%20Anim (Components|SkeletalMesh|GetAnimInstance _weapon_mesh)))

(event EventDestroyed
  (bind _firing_audio (Variables|Default|GetFiring%20Audio))
  ;[1 1 1] Fire bullets
  (Utilities|IsValid _firing_audio
    (:Is%20Valid
      (Components|DestroyComponent _firing_audio))))

(event EventTick
  (params (DeltaSeconds :type Float%20%28single-precision%29))
  (bind _targeting_camera (Variables|Default|GetTargeting%20Camera))
  (bind _arrow (Variables|Default|GetArrow))
  ;[1 1 1] Animate glowing barrels
  (if (Variables|Default|GetFiring%20Is%20Held)
    (Variables|Default|SetGlow (Math|Interpolation|FInterptoConstant (Variables|Default|GetGlow) 1.1 DeltaSeconds 0.05))
    (else
      (bind _output_get (Variables|Default|SetGlow (Math|Interpolation|FInterptoConstant (Variables|Default|GetGlow) 0.0 DeltaSeconds 0.12)))))
  (Rendering|Material|SetScalarParameterValue (Variables|Default|GetMaterial%20Inst) "Emis Power" (Math|Float|Clamp(Float) (- _output_get 0.1)) :!class /Script/Engine.MaterialInstanceDynamic)
  ;[1 1 1] Fine tune aming to camera target
  (Utilities|IsValid _targeting_camera
    (:Is%20Valid
      (bind _result_location (CallFunction|FS1TraceCheck _targeting_camera (Utilities|Array|MakeArray (Game|GetPlayerCharacter 0)) "TraceTypeQuery1"))
      (Transformation|SetWorldRotation _arrow (Class|KismetMathLibrary|RInterptoConstant (Transformation|GetWorldRotation (Variables|Default|GetRef_Arrow)) (Math|Rotator|FindLookatRotation (Transformation|GetWorldLocation _arrow) _result_location) 1.0 6.0) false false))
    (:Is%20Not%20Valid
      (Transformation|SetRelativeRotation (Variables|Default|GetArrow) "90.000000, 0, 0" false false))))

(event EventFS1UpdateMaterial
  (params (Armor :type Material%20Interface%20Object%20Reference) (Armor_2 :type Material%20Interface%20Object%20Reference) (Wings :type Material%20Interface%20Object%20Reference) (Minigun :type Material%20Interface%20Object%20Reference) (Railgun :type Material%20Interface%20Object%20Reference) (Rails :type Material%20Interface%20Object%20Reference) (Missiles :type Material%20Interface%20Object%20Reference))
  (bind _weapon_mesh (Variables|Default|GetWeapon_Mesh))
  ;[1 1 1] Recieve updates to material
  (Rendering|Material|SetMaterial _weapon_mesh 0 Minigun)
  (bind _returnvalue (Rendering|Material|CreateDynamicMaterialInstance _weapon_mesh 0 Minigun "None" :!class /Script/Engine.PrimitiveComponent))
  (bind _output_get (Variables|Default|SetMaterial%20Inst _returnvalue))
  (Rendering|Material|SetScalarParameterValue _output_get "Emis Power" (Variables|Default|GetGlow) :!class /Script/Engine.MaterialInstanceDynamic))

(event EventFS1OutlinedMeshes
  (params (Use%20Outlined%20Meshes :type Boolean))
  ;[1 1 1] Update to outlined meshes
  (Components|SkinnedMesh|SetSkinnedAssetandUpdate (Variables|Default|GetWeapon_Mesh) (select Use%20Outlined%20Meshes "/Game/Flight_Suit_1/Meshes/Weapons/Outlined/FS1_Podded_Minigun_Outlined_SK.FS1_Podded_Minigun_Outlined_SK" "/Game/Flight_Suit_1/Meshes/Weapons/FS1_Podded_Minigun_SK.FS1_Podded_Minigun_SK") true))

(event EventFunctionFireWeapon
  (params (FiringHeld :type Boolean) (HitScan :type Boolean) (ReadyFiring :type Boolean) (CameraComponent :type Scene%20Component%20Object%20Reference))
  ;[1 1 1] Recieve updates to fire
  (bind _output_get (Variables|Default|SetFiring%20Is%20Held FiringHeld))
  (bind _output_get_2 (Variables|Default|SetReadied%20To%20Fire ReadyFiring))
  (Variables|Default|SetTargeting%20Camera CameraComponent)
  ;[1 1 1] Fire bullets
  (Class|FS1BPI|FS1Fire(Message) (Variables|Default|GetGun%20Anim) _output_get false _output_get_2 CameraComponent "NewEnumerator9" "Target")
  (Class|TGBaseWeapon|CheckforHitScan HitScan)
  (if _output_get
    (if (not (Variables|Default|GetFiring))
      (Variables|Default|SetFiring true)
      (Utilities|FlowControl|Sequence
        (:then_0
          (Utilities|Time|SetTimerbyEvent (delegate Custom|Next%20Round%20Ready) (/ 1.0 (Variables|Default|GetBullets%20Per%20Second))))
        (:then_1
          (goto _label Close))
        (:then_2
          (Utilities|IsValid (Variables|Default|GetFiring%20Audio)
            (:Is%20Valid
              (Components|DestroyComponent (Variables|Default|GetFiring%20Audio)))
            (:Is%20Not%20Valid
              _))
          (bind _returnvalue (Audio|SpawnSoundAttached "/Game/Flight_Suit_1/Audio/FS1_Minigun_Firing_1_Cue.FS1_Minigun_Firing_1_Cue" (Variables|Default|GetArrow) "None" "0, 0, 0" "0, 0, 0" "KeepRelativeOffset" true 0.9 0.9 0.0 "/Game/Flight_Suit_1/Audio/20M_Attenuation.20M_Attenuation" 0))
          (bind _output_get_3 (Variables|Default|SetFiring%20Audio _returnvalue))
          (Audio|Components|Audio|FadeIn _output_get_3 0.1 0.9 0.0 "Linear" :!class /Script/Engine.AudioComponent))))
    (else
      (Variables|Default|SetFiring false)
      (Utilities|FlowControl|Sequence
        (:then_0
          (goto _label Open))
        (:then_1
          (Utilities|IsValid (Variables|Default|GetFiring%20Audio)
            (:Is%20Valid
              (Audio|Components|Audio|FadeOut (Variables|Default|GetFiring%20Audio) 0.1 0.0 "Linear" :!class /Script/Engine.AudioComponent)
              (Utilities|FlowControl|Delay 0.1)
              (Utilities|FlowControl|Gate true :!label _label
                (:Exit
                  (Utilities|IsValid (Variables|Default|GetFiring%20Audio)
                    (:Is%20Valid
                      (Components|DestroyComponent (Variables|Default|GetFiring%20Audio)))))))))))))

(fn ConstructionScript)

(fn GetIgnores
  (bind _ignore_actors (Class|FS1BPI|GetIgnores(Message) (Components|GetOwner)))
  (return _ignore_actors))