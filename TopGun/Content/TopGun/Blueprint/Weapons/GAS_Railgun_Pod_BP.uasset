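; Podded railgun weapon that fires rounds on a timed cooldown while the fire input is held.
; Each shot triggers the gun's anim instance, sound and muzzle particles, with the round actor spawned only on the server.
; Shots add capped barrel glow that decays on Tick, with a second smoothed value driving the material's emissive power.
; Events swap the weapon material or outlined mesh, and GetIgnores relays the owner's ignore list.
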(event Custom|Next%20Round%20Ready
  ;[1 1 1] Fire bullets
  (Variables|Default|SetCan%20Fire true))

(event EventBeginPlay
  (bind _weapon_mesh (Variables|Default|GetWeapon_Mesh))
  ;[1 1 1] Set weapon material on start
  (bind _returnvalue (Rendering|Material|CreateDynamicMaterialInstance _weapon_mesh 0 0 "None" :!class /Script/Engine.PrimitiveComponent))
  (bind _output_get (Variables|Default|SetMaterial%20Inst _returnvalue))
  (Rendering|Material|SetScalarParameterValue _output_get "Emis Power" (Variables|Default|GetGlow) :!class /Script/Engine.MaterialInstanceDynamic)
  (Variables|Default|SetGun%20Anim (Components|SkeletalMesh|GetAnimInstance _weapon_mesh)))

(event EventFS1OutlinedMeshes
  (params (Use%20Outlined%20Meshes :type Boolean))
  (Components|SkinnedMesh|SetSkinnedAssetandUpdate (Variables|Default|GetWeapon_Mesh) (select Use%20Outlined%20Meshes "/Game/Flight_Suit_1/Meshes/Weapons/Outlined/FS1_Podded_Railgun_Outlined_SK.FS1_Podded_Railgun_Outlined_SK" "/Game/Flight_Suit_1/Meshes/Weapons/FS1_Podded_Railgun_SK.FS1_Podded_Railgun_SK") true))

(event EventTick
  (params (DeltaSeconds :type Float%20%28single-precision%29))
  ;[1 1 1] Animate glowing barrels
  (bind _output_get (Variables|Default|SetGlow (Math|Interpolation|FInterptoConstant (Variables|Default|GetGlow) 0.0 DeltaSeconds 0.2)))
  (bind _output_get_2 (Variables|Default|SetVis%20Glow (Math|Interpolation|FInterptoConstant (Variables|Default|GetVis%20Glow) _output_get DeltaSeconds 1.5)))
  (Rendering|Material|SetScalarParameterValue (Variables|Default|GetMaterial%20Inst) "Emis Power" _output_get_2 :!class /Script/Engine.MaterialInstanceDynamic))

(event EventFS1Fire
  (params (Firing%20Held :type Boolean) (Firing%20Mode%20Update :type Boolean) (Ready%20Firing :type Boolean) (Camera%20Reference :type Scene%20Component%20Object%20Reference) (Slots%20Affected%20By%20Fire :type FS1_Weapon_Slots_Enum%20Enum :default "NewEnumerator0") (Targeting%20Tag :type Name :default "None"))
  (bind _gun_anim (Variables|Default|GetGun%20Anim))
  ;[1 1 1] Recieve updates to fire
  (bind _output_get (Variables|Default|SetFiring%20Is%20Held (stale EventFunctionFireWeapon FiringHeld)))
  (Variables|Default|SetReadied%20To%20Fire (stale EventFunctionFireWeapon ReadyFiring))
  (Variables|Default|SetTargeting%20Camera (stale EventFunctionFireWeapon CameraComponent))
  ;[1 1 1] Fire bullets
  (if (Variables|Default|GetCan%20Fire)
    (if _output_get
      (Variables|Default|SetGlow (Math|Float|Clamp(Float) (+ (Variables|Default|GetGlow) 0.35) 0.0 1.2))
      (Utilities|FlowControl|Sequence
        (:then_0
          (Class|FS1BPI|FS1Fire(Message) _gun_anim true false false 0 "NewEnumerator9" "Target")
          (Variables|Default|SetCan%20Fire false)
          (Utilities|Time|SetTimerbyEvent (delegate Custom|Next%20Round%20Ready) 0.5)
          (if (Networking|IsServer)
            (Game|SpawnActorfromClass "/Game/Flight_Suit_1/Blueprints/Weapons/Projectiles/FS1_Railgun_Round_BP.FS1_Railgun_Round_BP_C" (Transformation|GetWorldTransform (Variables|Default|GetArrow)) "AlwaysSpawn" "OverrideRootScale" self 0))
          (Audio|SpawnSoundAttached "/Game/Flight_Suit_1/Audio/FS1_Railgun_Fire_1_Cue.FS1_Railgun_Fire_1_Cue" (Variables|Default|GetArrow) "None" "0, 0, 0" "0, 0, 0" "KeepRelativeOffset" false 1.0 1.0 0.0 0 0)
          (Effects|SpawnEmitterAttached "/Game/Flight_Suit_1/Particles/Railgun_Firing_PS.Railgun_Firing_PS" (Variables|Default|GetArrow) "None" "0, 0, 0" "0, 0, 0" "0.300000,0.300000,0.300000"))
        (:then_1
          (Utilities|FlowControl|Delay 0.1)
          (Class|FS1BPI|FS1Fire(Message) _gun_anim false false false 0 "NewEnumerator9" "Target"))))))

(event EventFS1UpdateMaterial
  (params (Armor :type Material%20Interface%20Object%20Reference) (Armor_2 :type Material%20Interface%20Object%20Reference) (Wings :type Material%20Interface%20Object%20Reference) (Minigun :type Material%20Interface%20Object%20Reference) (Railgun :type Material%20Interface%20Object%20Reference) (Rails :type Material%20Interface%20Object%20Reference) (Missiles :type Material%20Interface%20Object%20Reference))
  (bind _weapon_mesh (Variables|Default|GetWeapon_Mesh))
  ;[1 1 1] Recieve updates to material
  (Rendering|Material|SetMaterial _weapon_mesh 0 Railgun)
  (bind _returnvalue (Rendering|Material|CreateDynamicMaterialInstance _weapon_mesh 0 Railgun "None" :!class /Script/Engine.PrimitiveComponent))
  (bind _output_get (Variables|Default|SetMaterial%20Inst _returnvalue))
  (Rendering|Material|SetScalarParameterValue _output_get "Emis Power" (Variables|Default|GetGlow) :!class /Script/Engine.MaterialInstanceDynamic))

(event EventFunctionFireWeapon
  (params (FiringHeld :type Boolean) (ReadyFiring :type Boolean) (CameraComponent :type Scene%20Component%20Object%20Reference))
  (bind _gun_anim (Variables|Default|GetGun%20Anim))
  ;[1 1 1] Recieve updates to fire
  (bind _output_get (Variables|Default|SetFiring%20Is%20Held FiringHeld))
  (Variables|Default|SetReadied%20To%20Fire ReadyFiring)
  (Variables|Default|SetTargeting%20Camera CameraComponent)
  ;[1 1 1] Fire bullets
  (if (Variables|Default|GetCan%20Fire)
    (if _output_get
      (Variables|Default|SetGlow (Math|Float|Clamp(Float) (+ (Variables|Default|GetGlow) 0.35) 0.0 1.2))
      (Utilities|FlowControl|Sequence
        (:then_0
          (Class|FS1BPI|FS1Fire(Message) _gun_anim true false false 0 "NewEnumerator9" "Target")
          (Variables|Default|SetCan%20Fire false)
          (Utilities|Time|SetTimerbyEvent (delegate Custom|Next%20Round%20Ready) 0.5)
          (if (Networking|IsServer)
            (Game|SpawnActorfromClass "/Game/Flight_Suit_1/Blueprints/Weapons/Projectiles/FS1_Railgun_Round_BP.FS1_Railgun_Round_BP_C" (Transformation|GetWorldTransform (Variables|Default|GetArrow)) "AlwaysSpawn" "OverrideRootScale" self 0))
          (Audio|SpawnSoundAttached "/Game/Flight_Suit_1/Audio/FS1_Railgun_Fire_1_Cue.FS1_Railgun_Fire_1_Cue" (Variables|Default|GetArrow) "None" "0, 0, 0" "0, 0, 0" "KeepRelativeOffset" false 1.0 1.0 0.0 0 0)
          (Effects|SpawnEmitterAttached "/Game/Flight_Suit_1/Particles/Railgun_Firing_PS.Railgun_Firing_PS" (Variables|Default|GetArrow) "None" "0, 0, 0" "0, 0, 0" "0.300000,0.300000,0.300000"))
        (:then_1
          (Utilities|FlowControl|Delay 0.1)
          (Class|FS1BPI|FS1Fire(Message) _gun_anim false false false 0 "NewEnumerator9" "Target"))))))

(fn ConstructionScript)

(fn GetIgnores
  (bind _ignore_actors (Class|FS1BPI|GetIgnores(Message) (Components|GetOwner)))
  (return _ignore_actors))