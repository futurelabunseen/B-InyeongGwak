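; Dual missile rail weapon Blueprint that fires two light missiles, one per fire message while firing is held.
; Each shot hides the next rail-mounted mesh, and only the server spawns the missile actor at its transform, passing camera, velocity source and material.
; Reload restores both meshes and resets the counter.
; Events also swap rail and missile materials and toggle outlined meshes, though M1 always gets the plain mesh.
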(event EventBeginPlay
  ;[1 1 1] Set weapon material on start
  (bind _returnvalue (Rendering|Material|CreateDynamicMaterialInstance (Variables|Default|GetFS1_Dual_Rail_Main_SM) 0 0 "None" :!class /Script/Engine.PrimitiveComponent))
  (Variables|Default|SetMaterial%20Inst _returnvalue))

(event EventFS1Reload
  (params (Weapon%20To%20Reload :type FS1_Weapon_Slots_Enum%20Enum :default "NewEnumerator0"))
  ;[1 1 1] Reload Rail
  (for _array_element (Utilities|Array|MakeArray (Variables|Default|GetM1) (Variables|Default|GetM2))
    (Rendering|SetVisibility _array_element true false))
  (Variables|Default|SetMissile%20To%20Fire 0))

(event EventTick
  (params (DeltaSeconds :type Float%20%28single-precision%29))
  ;[1 1 1] Animate glowing barrels
)

(event EventFS1UpdateMaterial
  (params (Armor :type Material%20Interface%20Object%20Reference) (Armor_2 :type Material%20Interface%20Object%20Reference) (Wings :type Material%20Interface%20Object%20Reference) (Minigun :type Material%20Interface%20Object%20Reference) (Railgun :type Material%20Interface%20Object%20Reference) (Rails :type Material%20Interface%20Object%20Reference) (Missiles :type Material%20Interface%20Object%20Reference))
  (bind _fs1_dual_rail_main_sm (Variables|Default|GetFS1_Dual_Rail_Main_SM))
  ;[1 1 1] Recieve updates to material
  (Variables|Default|SetMissiles%20Mat Missiles)
  (Rendering|Material|SetMaterial _fs1_dual_rail_main_sm 0 Rails)
  (bind _returnvalue (Rendering|Material|CreateDynamicMaterialInstance _fs1_dual_rail_main_sm 0 Rails "None" :!class /Script/Engine.PrimitiveComponent))
  (Variables|Default|SetMaterial%20Inst _returnvalue)
  (for _array_element (Utilities|Array|MakeArray (Variables|Default|GetM1) (Variables|Default|GetM2))
    (Rendering|Material|SetMaterial _array_element 0 Missiles)))

(event EventFS1OutlinedMeshes
  (params (Use%20Outlined%20Meshes :type Boolean))
  ;[1 1 1] Update to outlined meshes
  (Components|StaticMesh|SetStaticMesh (Variables|Default|GetFS1_Dual_Rail_Main_SM) (select Use%20Outlined%20Meshes "/Game/Flight_Suit_1/Meshes/Weapons/Outlined/FS1_Dual_Rail_Main_Outlined_SM.FS1_Dual_Rail_Main_Outlined_SM" "/Game/Flight_Suit_1/Meshes/Weapons/FS1_Dual_Rail_Main_SM.FS1_Dual_Rail_Main_SM"))
  (Components|StaticMesh|SetStaticMesh (Variables|Default|GetM1) (select false "/Game/Flight_Suit_1/Meshes/Weapons/Outlined/FS1_Light_Missile_Outlined_SM.FS1_Light_Missile_Outlined_SM" "/Game/Flight_Suit_1/Meshes/Weapons/FS1_Light_Missile_SM.FS1_Light_Missile_SM"))
  (Components|StaticMesh|SetStaticMesh (Variables|Default|GetM2) (select Use%20Outlined%20Meshes "/Game/Flight_Suit_1/Meshes/Weapons/Outlined/FS1_Light_Missile_Outlined_SM.FS1_Light_Missile_Outlined_SM" "/Game/Flight_Suit_1/Meshes/Weapons/FS1_Light_Missile_SM.FS1_Light_Missile_SM")))

(event EventFunctionFireWeapon
  (params (FiringHeld :type Boolean) (HitScan :type Boolean) (ReadyFiring :type Boolean) (CameraComponent :type Scene%20Component%20Object%20Reference))
  (bind _missile_to_fire (Variables|Default|GetMissile%20To%20Fire))
  (bind _m2 (Variables|Default|GetM2))
  (bind _m1 (Variables|Default|GetM1))
  (bind _array (Utilities|Array|MakeArray _m1 _m2))
  (bind _output (Utilities|Array|Get(acopy) _array _missile_to_fire))
  ;[1 1 1] Recieve updates to fire
  (Utilities|String|LogString "Hello")
  (bind _output_get (Variables|Default|SetFiring%20Is%20Held FiringHeld))
  (Variables|Default|SetReadied%20To%20Fire ReadyFiring)
  (bind _output_get_2 (Variables|Default|SetTarget%20Tag "None"))
  ;[1 1 1] Fire Next Missile
  (if _output_get
    (if (< _missile_to_fire 2)
      (Rendering|SetVisibility _output false false)
      (if (Networking|IsServer)
        (bind _returnvalue (Game|SpawnActorfromClass "/Game/Flight_Suit_1/Blueprints/Weapons/Projectiles/FS1_Missile_Light_BP.FS1_Missile_Light_BP_C" (Transformation|GetWorldTransform _output) "AlwaysSpawn" "OverrideRootScale" self "/Game/Flight_Suit_1/Demo/Particles/P_Explosion_PS.P_Explosion_PS" "/Game/Flight_Suit_1/Demo/Audio/Explosion_Cue.Explosion_Cue" (Components|GetOwner CameraComponent) 0))
        (Utilities|IsValid _returnvalue
          (:Is%20Valid
            (Class|FS1BPI|FS1Fire(Message) _returnvalue true false false CameraComponent "NewEnumerator9" _output_get_2)
            (Class|FS1BPI|FS1UpdateMaterial(Message) _returnvalue 0 0 0 0 0 0 (Variables|Default|GetMissiles%20Mat)))
          (:Is%20Not%20Valid
            _)))
      (Math|Integer|IncrementInt _missile_to_fire))))

(fn ConstructionScript)

(fn GetIgnores
  (bind _ignore_actors (Class|FS1BPI|GetIgnores(Message) (Components|GetOwner)))
  (return _ignore_actors))