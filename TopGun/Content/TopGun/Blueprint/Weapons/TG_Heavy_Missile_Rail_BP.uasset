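; Heavy missile rail weapon for aircraft in TopGun that launches a single heavy missile per reload.
; On a fire update it hides the mounted missile mesh and the server spawns a missile actor at that transform, passing the camera, its owner as velocity source and the missile material.
; Reload restores the mesh and re-arms the rail.
; Other events swap rail and missile materials or switch to outlined meshes.
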(event EventBeginPlay
  ;[1 1 1] Set weapon material on start
  (bind _returnvalue (Rendering|Material|CreateDynamicMaterialInstance (Variables|Default|GetFS1_Heavy_Rail_Main_SM) 0 0 "None" :!class /Script/Engine.PrimitiveComponent))
  (Variables|Default|SetMaterial%20Inst _returnvalue))

(event EventFS1Reload
  (params (Weapon%20To%20Reload :type FS1_Weapon_Slots_Enum%20Enum :default "NewEnumerator0"))
  ;[1 1 1] Reload Rail
  (Rendering|SetVisibility (Variables|Default|GetMissile_SM) true false)
  (Variables|Default|SetMissile%20Fired false))

(event EventTick
  (params (DeltaSeconds :type Float%20%28single-precision%29)))

(event EventFS1UpdateMaterial
  (params (Armor :type Material%20Interface%20Object%20Reference) (Armor_2 :type Material%20Interface%20Object%20Reference) (Wings :type Material%20Interface%20Object%20Reference) (Minigun :type Material%20Interface%20Object%20Reference) (Railgun :type Material%20Interface%20Object%20Reference) (Rails :type Material%20Interface%20Object%20Reference) (Missiles :type Material%20Interface%20Object%20Reference))
  (bind _fs1_heavy_rail_main_sm (Variables|Default|GetFS1_Heavy_Rail_Main_SM))
  ;[1 1 1] Recieve updates to material
  (Variables|Default|SetMissiles%20Mat Missiles)
  (Rendering|Material|SetMaterial _fs1_heavy_rail_main_sm 0 Rails)
  (bind _returnvalue (Rendering|Material|CreateDynamicMaterialInstance _fs1_heavy_rail_main_sm 0 Rails "None" :!class /Script/Engine.PrimitiveComponent))
  (Variables|Default|SetMaterial%20Inst _returnvalue)
  (Rendering|Material|SetMaterial (Variables|Default|GetMissile_SM) 0 Missiles))

(event EventFS1OutlinedMeshes
  (params (Use%20Outlined%20Meshes :type Boolean))
  ;[1 1 1] Update to outlined meshes
  (Components|StaticMesh|SetStaticMesh (Variables|Default|GetFS1_Heavy_Rail_Main_SM) (select Use%20Outlined%20Meshes "/Game/Flight_Suit_1/Meshes/Weapons/Outlined/FS1_Heavy_Rail_Main_Outlined_SM.FS1_Heavy_Rail_Main_Outlined_SM" "/Game/Flight_Suit_1/Meshes/Weapons/FS1_Heavy_Rail_Main_SM.FS1_Heavy_Rail_Main_SM"))
  (Components|StaticMesh|SetStaticMesh (Variables|Default|GetMissile_SM) (select Use%20Outlined%20Meshes "/Game/Flight_Suit_1/Meshes/Weapons/Outlined/FS1_Heavy_Missile_Outlined_SM.FS1_Heavy_Missile_Outlined_SM" "/Game/Flight_Suit_1/Meshes/Weapons/FS1_Heavy_Missile_SM.FS1_Heavy_Missile_SM")))

(event EventFunctionFireWeapon
  (params (FiringHeld :type Boolean) (HitScan :type Boolean) (ReadyFiring :type Boolean) (CameraComponent :type Scene%20Component%20Object%20Reference))
  (bind _missile_sm (Variables|Default|GetMissile_SM))
  ;[1 1 1] Recieve updates to fire
  (bind _output_get (Variables|Default|SetFiring%20Is%20Held FiringHeld))
  (Variables|Default|SetReadied%20To%20Fire ReadyFiring)
  (bind _output_get_2 (Variables|Default|SetTarget%20Tag "None"))
  ;[1 1 1] Spawn missile
  (if _output_get
    (if (not (Variables|Default|GetMissile%20Fired))
      (Variables|Default|SetMissile%20Fired true)
      (Rendering|SetVisibility _missile_sm false false)
      (if (Networking|IsServer)
        (bind _returnvalue (Game|SpawnActorfromClass "/Game/Flight_Suit_1/Blueprints/Weapons/Projectiles/FS1_Missile_Heavy_BP.FS1_Missile_Heavy_BP_C" (Transformation|GetWorldTransform _missile_sm) "AlwaysSpawn" "OverrideRootScale" self "/Game/Flight_Suit_1/Demo/Particles/P_Explosion_PS.P_Explosion_PS" "/Game/Flight_Suit_1/Demo/Audio/Explosion_Cue.Explosion_Cue" (Components|GetOwner CameraComponent) 0))
        (Class|FS1BPI|FS1Fire(Message) _returnvalue true false false CameraComponent "NewEnumerator9" _output_get_2)
        (Class|FS1BPI|FS1UpdateMaterial(Message) _returnvalue 0 0 0 0 0 0 (Variables|Default|GetMissiles%20Mat))))))

(fn ConstructionScript)

(fn GetIgnores
  (bind _ignore_actors (Class|FS1BPI|GetIgnores(Message) (Components|GetOwner)))
  (return _ignore_actors))