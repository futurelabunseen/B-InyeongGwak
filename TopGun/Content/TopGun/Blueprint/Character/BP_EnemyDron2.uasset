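; BP_EnemyDron2 is an AI enemy drone that hunts the player and fires a dual missile rail weapon.
; On BeginPlay it passes the BT_Chase behavior tree and the player pawn as sensing target to its My_AIC controller.
; Firing runs separately from the AI: a looping Delay chain started from Tick logs and sends fire messages to the missile rail with its camera, with no target check.
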(event EventBeginPlay
  ;[1 1 1] Setup the AI Controller with the Target Pawn and the Behavior Tree to use
  (bind _asmy_aic (Utilities|Casting|CastToMy_AIC (AI|GetAIController self)))
  (Default|SetupAIC _asmy_aic "/Game/FlyingAI/AI/BT_Chase.BT_Chase" (Game|Player|GetPlayerPawn 0)))

(event Collision|EventActorBeginOverlap
  (params (OtherActor :type Actor%20Object%20Reference)))

(event EventTick
  (params (DeltaSeconds :type Float%20%28single-precision%29))
  (Utilities|FlowControl|Delay 3.0 :!label _label)
  (Utilities|String|LogString "Fire")
  (Class|TGWeaponInterface|FunctionFireWeapon(Message) (Variables|Default|GetTG_Dual_Missile_Rail_BP) true false true (Variables|Default|GetCamera))
  (Utilities|FlowControl|Delay 3.0)
  (goto _label))

(fn ConstructionScript)