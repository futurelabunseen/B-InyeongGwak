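; Temporary player character that wears an FS1 flight suit as a child actor and drives it through messages.
; The construction script caches the suit, attaches it to the character mesh, passes outline settings and remaps bone names and offsets for the UE5 skeleton.
; Left mouse press turns on aiming and, when weapon firing is enabled, sends the suit a fire message with the follow camera.
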(event Input|MouseEvents|LeftMouseButton
  (params (Key :type Key%20Structure :default "None"))
  (:Pressed
    (bind _output_get (Variables|Weapons|SetLMB%20Down true))
    (bind _output_get_2 (Variables|Weapons|SetAiming%20Mode true))
    (Utilities|FlowControl|Sequence
      (:then_0
        (if (Variables|Weapons|GetFire%20Weps%201)
          (Class|FS1BPI|FS1Fire(Message) (Variables|Default|GetFlight_Suit_1_Actor) _output_get false _output_get_2 (Variables|Default|GetFollowCamera) "NewEnumerator6" "Target"))))))

(fn ConstructionScript
  ;[1 1 1] Save reference to flight suit, and set the parent mesh it will follow.
  (bind _asfs1_bp (Utilities|Casting|CastToFS1_BP (Variables|/Script/Engine.ChildActorComponent|GetChildActor (Variables|Default|GetFlight_Suit_1_Actor))))
  (bind _output_get (Variables|Default|SetFlight%20Suit%20Actor _asfs1_bp))
  (Class|FS1BPI|FS1SetParentMesh(Message) _output_get (Variables|Character|GetMesh))
  ;[1 1 1] Set to use UE5 skeleton meshes and spine offset (spine_05 is closest to old Spine_03, but slightly higher relative to it on the mesh), Also foot offsets, since they too changed their bones pivot point a bit along with the calves. If you need your own basic tweaks, just open the FS1_BPI, and find the "FS1 Set Bone Names" message and add the new translations/rotations you want. Then you can save those in the set bones event node in the FS1_BP and then use those to make the adjustments to the meshes when it connects them to the parent.
  (Class|FS1BPI|FS1OutlinedMeshes(Message) (Variables|Default|GetFlight%20Suit%20Actor) (Variables|Default|GetOutlined%20Meshes))
  (Class|FS1BPI|FS1SetBoneNames(Message) (Variables|Default|GetFlight%20Suit%20Actor) "Thigh_r" "Thigh_l" "Calf_L" "Calf_R" "Pelvis" "Spine_05" "Spine_05" "upperarm_l" "upperarm_r" "lowerarm_l" "lowerarm_r" "head" "foot_l" "foot_r" "ball_l" "Ball_r" "-2.750000,0.000000,0.000000" "-2.750000, 0, 0" "4.000000, 0, 0" "-4.000000, 0, 0" "6.000000, 0, 0" "-6.000000, 0, 0"))